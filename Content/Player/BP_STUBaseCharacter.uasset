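; Base player character Blueprint that lets the player switch between its default camera and a first-person camera.
; The Change Person Perspective input checks whether CameraComponent is active, then activates one camera component and deactivates the other.
; Actor overlaps print the other actor's name, while BeginPlay, Hit, Tick and the construction script are empty.
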(event EventBeginPlay)

(event Collision|EventActorBeginOverlap
  (params (OtherActor :type Actor%20Object%20Reference))
  (Development|PrintString (Utilities|GetDisplayName OtherActor)))

(event EventTick
  (params (DeltaSeconds :type Float%20%28single-precision%29)))

(event Collision|EventHit
  (params (MyComp :type Primitive%20Component%20Object%20Reference) (Other :type Actor%20Object%20Reference) (OtherComp :type Primitive%20Component%20Object%20Reference) (bSelfMoved :type Boolean) (HitLocation :type Vector :default "0, 0, 0") (HitNormal :type Vector :default "0, 0, 0") (NormalImpulse :type Vector :default "0, 0, 0") (Hit :type Hit%20Result%20Structure%20%28by%20ref%29)))

(event Input|ActionEvents|InputActionChangePersonPerspective
  (params (Key :type Key%20Structure :default "None"))
  (bind _fppcameracomponent (Variables|Default|GetFPPCameraComponent))
  (bind _cameracomponent (Variables|Default|GetCameraComponent))
  (:Pressed
    (if (Components|Activation|IsActive (Variables|Default|GetCameraComponent))
      (Components|Activation|SetActive _fppcameracomponent true false)
      (Components|Activation|SetActive _cameracomponent false false)
      (else
        (Components|Activation|SetActive _fppcameracomponent false false)
        (Components|Activation|SetActive _cameracomponent true false)))))

(fn ConstructionScript)